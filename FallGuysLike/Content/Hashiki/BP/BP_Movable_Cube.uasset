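; BP_Movable_Cube is a cube actor that blinks between a normal and a light blue material.
; On BeginPlay it creates a dynamic instance of the base blue material and starts a looping one-second timer on ToggleMaterial.
; ToggleMaterial swaps the two material assets and flips IsEmissive, so the dynamic instance is never used afterwards.
; Despite the name, this graph contains no movement logic.
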(event `self.ReceiveBeginPlay`
  (`PrimitiveComponent.CreateDynamicMaterialInstance` (`self.Cube`) 0 "/Game/Hashiki/Material/M_Movable_Blue.M_Movable_Blue" "None")
  (`KismetSystemLibrary.K2_SetTimer` null "ToggleMaterial" 1.0 true))

(fn `ToggleMaterial`
  (if (`self.IsEmissive`)
    (`PrimitiveComponent.SetMaterial` (`self.Cube`) 0 "/Game/Hashiki/Material/M_Movable_Blue.M_Movable_Blue")
    (bind _output_get (set `self.IsEmissive` false))
    (else
      (`PrimitiveComponent.SetMaterial` (`self.Cube`) 0 "/Game/Hashiki/Material/M_Movable_Blue_Light.M_Movable_Blue_Light")
      (bind _output_get_2 (set `self.IsEmissive` true)))))

(fn `UserConstructionScript`)